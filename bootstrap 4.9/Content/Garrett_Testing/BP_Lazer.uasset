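; Laser beam actor that stretches from its origin to the first qualifying mirror detector or wall ahead of it.
; When flagged as the initial laser, it traces forward shortly after BeginPlay with a persistently drawn multi-object trace, stopping at a "Detector"-tagged mirror component or "Wall"-tagged actor.
; A while loop then increments the pivot's Y scale until the beam's end nears the impact point.
; ResetSize restores unit scale.
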(event `self.ReceiveBeginPlay`
  (if (`self.isInitialLazer`)
    (`KismetSystemLibrary.Delay` 0.2)
    (`self.Project Lazer Path`)))

(event `self.ReceiveActorBeginOverlap`
  (params (OtherActor :type "Actor Object Reference")))

(event `self.ReceiveTick`
  (params (DeltaSeconds :type "Float (single-precision)")))

(event `ScaleAlongPath`
  (params (`Destination Location` :type "Vector Structure"))
  (while (>= (`KismetMathLibrary.VSize` (- `Destination Location` (`SceneComponent.K2_GetComponentLocation` (`self.EndOfLazer`)))) 10.0)
    (`SceneComponent.SetWorldScale3D` (`self.LazerScalePivotPoint`) (+ (`SceneComponent.K2_GetComponentScale` (`self.LazerScalePivotPoint`)) (0.0 0.2 0.0)))))

(event `Project Lazer Path`
  (bind _returnvalue (`self.K2_GetActorLocation`))
  (bind _outhits (`KismetSystemLibrary.LineTraceMultiForObjects` :`Start` _returnvalue :`End` (+ (* (`self.GetActorForwardVector`) 50000.0) _returnvalue) :`ObjectTypes` (`|MakeArray` "ObjectTypeQuery1" "ObjectTypeQuery2" :!type "EObjectTypeQuery Enum") :`DrawDebugType` "Persistent"))
  (for _array_element _outhits :!label _label
    (bind (_bblockinghit _binitialoverlap _time _location _impactpoint _normal _impactnormal _physmat _hitactor _hitcomponent) (`GameplayStatics.BreakHitResult` _array_element))
    (if (`KismetSystemLibrary.IsValid` _hitactor)
      (if (or (`KismetMathLibrary.ClassIsChildOf` (`GameplayStatics.GetObjectClass` _hitactor) "/Game/Garrett_Testing/BP_MirrorHorizontal.BP_MirrorHorizontal_C") (`KismetMathLibrary.ClassIsChildOf` (`GameplayStatics.GetObjectClass` _hitactor) "/Game/Garrett_Testing/BP_Mirror_Vertical.BP_Mirror_Vertical_C"))
        (if (`ActorComponent.ComponentHasTag` _hitcomponent "Detector")
          (`self.Break Loop`)
          (`self.ScaleAlongPath` _impactpoint :!label _label_2))
        (elif (`self.ActorHasTag` _hitactor "Wall")
          (`self.Break Loop`)
          (goto _label_2))))))

(event `Break Loop`
  (goto _label :!via `Break`))

(fn `ResetSize`
  (`SceneComponent.SetWorldScale3D` (`self.LazerScalePivotPoint`) (1.0 1.0 1.0)))

(fn `UserConstructionScript`)