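; BP_MirrorVertical is a laser-puzzle mirror that emits its own BP_Lazer beam when a laser hits it.
; The child-actor beam starts hidden and LazerDetector overlap reveals it, but end overlap leaves it visible because the hide call is unconnected.
; RotateLeft and RotateRight roll pivot and beam within limits, then reset beam size; the beam's step is hard-coded, the pivot's uses RotateAmount.
; EnableLazer and DisableLazer spawn and destroy a separate laser, uncalled here.
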(event `/Game/Garrett_Testing/BP_Mirror_OLD.ReceiveBeginPlay`
  (`|ExecutionSequence`
    (:`then_0`
      ;[1 1 1] Enable input events to be allowed in this actor
      (bind _asplayer_controller (cast `PlayerController` (`GameplayStatics.GetPlayerController` 0)))
      (`self.EnableInput` _asplayer_controller))
    (:`then_1`
      ;[1 1 1] Create an initial reference to be used in the future
      (bind _asthird_person_character (cast `/Game/ThirdPersonBP/Blueprints/ThirdPersonCharacter` (`GameplayStatics.GetPlayerCharacter` 0)))
      (set `self.thirdPersonCharRef` _asthird_person_character))
    (:`then_2`
      (`SceneComponent.SetVisibility` (`self.LazerActor`) false true))
    (:`then_3`
      (bind _asbp_lazer (cast `/Game/Garrett_Testing/BP_Lazer` (`ChildActorComponent.ChildActor` (`self.LazerActor`))))
      (set `self.myLazerRef` _asbp_lazer))))

(event `self.LazerDetector.OnComponentBeginOverlap`
  (params (OtherActor :type "Actor Object Reference") (OtherComp :type "PrimitiveComponent Object Reference") (OtherBodyIndex :type Integer) (bFromSweep :type Boolean) (SweepResult :type "HitResult Structure (by ref)"))
  ;[1 1 1] Checks in the overlapped actor is a lazer, if so, spawn a lazer at this mirror
  (if (`KismetMathLibrary.ClassIsChildOf` (`GameplayStatics.GetObjectClass` OtherActor) "/Game/Garrett_Testing/BP_Lazer.BP_Lazer_C")
    (`SceneComponent.SetVisibility` (`self.LazerActor`) true true)))

(event `self.LazerDetector.OnComponentEndOverlap`
  (params (OtherActor :type "Actor Object Reference") (OtherComp :type "PrimitiveComponent Object Reference") (OtherBodyIndex :type Integer))
  ;[1 1 1] Destroy the lazer when it leaves the mirror
  (if (`KismetMathLibrary.ClassIsChildOf` (`GameplayStatics.GetObjectClass` OtherActor) "/Game/Garrett_Testing/BP_Lazer.BP_Lazer_C")
    _))

(fn `DisableLazer`
  (`self.K2_DestroyActor` (`self.myLazer`))
  (`KismetSystemLibrary.PrintString` "destroyed"))

(fn `EnableLazer`
  ;[1 1 1] Spawn lazer with publicly set sizing, then immediately create a reference variable
  (bind _returnvalue (`|SpawnActorFromClass` "/Game/Garrett_Testing/BP_Lazer.BP_Lazer_C" (`SceneComponent.K2_GetComponentToWorld` (`self.LazerRefPoint`)) "AlwaysSpawn" "OverrideRootScale"))
  (set `self.myLazer` _returnvalue))

(fn `RotateLeft`
  (bind _mirrorrotationpivot (`self.MirrorRotationPivot`))
  ;[1 1 1] If the mirror rotation is greater than the minimum, rotate equal to the rotateAmount
  (if (>= (.roll (`SceneComponent.K2_GetComponentRotation` (`self.MirrorRotationPivot`))) (`self.rotateMin`))
    (`SceneComponent.K2_SetWorldRotation` (`self.LazerActor`) (`KismetMathLibrary.MakeRotator` (- (.roll (`SceneComponent.K2_GetComponentRotation` (`self.LazerActor`))) 15.0) (.pitch (`SceneComponent.K2_GetComponentRotation` (`self.LazerActor`))) (.yaw (`SceneComponent.K2_GetComponentRotation` (`self.LazerActor`)))) false false)
    (`SceneComponent.K2_SetWorldLocationAndRotation` (`self.MirrorRotationPivot`) (`SceneComponent.K2_GetComponentLocation` _mirrorrotationpivot) (`KismetMathLibrary.MakeRotator` (- (.roll (`SceneComponent.K2_GetComponentRotation` _mirrorrotationpivot)) (`self.rotateAmount`)) (.pitch (`SceneComponent.K2_GetComponentRotation` _mirrorrotationpivot)) (.yaw (`SceneComponent.K2_GetComponentRotation` _mirrorrotationpivot))) false false)
    (`/Game/Garrett_Testing/BP_Lazer.ResetSize` (`self.myLazerRef`))))

(fn `RotateRight`
  (bind _mirrorrotationpivot (`self.MirrorRotationPivot`))
  ;[1 1 1] If the mirror rotation is less than the maximum, rotate equal to the rotateAmount
  (if (<= (.roll (`SceneComponent.K2_GetComponentRotation` (`self.MirrorRotationPivot`))) (`self.rotateMax`))
    (`SceneComponent.K2_SetWorldRotation` (`self.LazerActor`) (`KismetMathLibrary.MakeRotator` (+ (.roll (`SceneComponent.K2_GetComponentRotation` (`self.LazerActor`))) 15.0) (.pitch (`SceneComponent.K2_GetComponentRotation` (`self.LazerActor`))) (.yaw (`SceneComponent.K2_GetComponentRotation` (`self.LazerActor`)))) false false)
    (`SceneComponent.K2_SetWorldLocationAndRotation` (`self.MirrorRotationPivot`) (`SceneComponent.K2_GetComponentLocation` _mirrorrotationpivot) (`KismetMathLibrary.MakeRotator` (+ (.roll (`SceneComponent.K2_GetComponentRotation` _mirrorrotationpivot)) (`self.rotateAmount`)) (.pitch (`SceneComponent.K2_GetComponentRotation` _mirrorrotationpivot)) (.yaw (`SceneComponent.K2_GetComponentRotation` _mirrorrotationpivot))) false false)
    (`/Game/Garrett_Testing/BP_Lazer.ResetSize` (`self.myLazerRef`))))

(fn `UserConstructionScript`)