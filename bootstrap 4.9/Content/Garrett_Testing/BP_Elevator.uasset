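; Elevator actor that travels vertically between floors marked by TargetPoint actors tagged with floor numbers.
; BeginPlay collects every TargetPoint and snaps the elevator to the starting floor.
; GoToFloor ignores calls while moving, otherwise finds the target tag and starts moving up or down.
; Movement re-triggers itself through short delays, stepping Z with sweep, accelerating near departure and decelerating near arrival by distance checks.
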(event `self.ReceiveBeginPlay`
  ;[1 1 1] Grab all floor target points and add them into an array
  (bind _outactors (`GameplayStatics.GetAllActorsOfClass` "/Script/Engine.TargetPoint"))
  (for _array_element _outactors
    (`KismetArrayLibrary.Array_Add` (`self.floorArray`) _array_element))
  ;[1 1 1] Teleports the elevator to the starting floor designated by the 'startingFloor' var
  (for _array_element_2 (`self.floorArray`)
    (if (`self.ActorHasTag` _array_element_2 (`KismetStringLibrary.Conv_StringToName` (`KismetStringLibrary.Conv_IntToString` (`self.startingFloor`))))
      (`self.K2_SetActorLocation` (`self.K2_GetActorLocation` _array_element_2))
      (set `self.currentFloor` (`self.startingFloor`))
      (set `self.currentFloorRef` _array_element_2))))

(event `Go To Floor`
  (params (`Floor to Go To` :type Integer))
  (if (not (`self.isMoving`))
    (`/Engine/EditorBlueprintResources/StandardMacros.CompareInt` `Floor to Go To` (`self.currentFloor`)
      (:`>`
        (for _array_element (`self.floorArray`)
          (if (`self.ActorHasTag` _array_element (`KismetStringLibrary.Conv_StringToName` (`KismetStringLibrary.Conv_IntToString` `Floor to Go To`)))
            (`|ExecutionSequence`
              (:`then_0`
                (break))
              (:`then_1`
                (set `self.targetFloorRef` _array_element)
                (set `self.targetFloor` `Floor to Go To`)
                (set `self.isMoving` true)
                (`self.Move Up`))))))
      (:`<`
        (for _array_element_2 (`self.floorArray`)
          (if (`self.ActorHasTag` _array_element_2 (`KismetStringLibrary.Conv_StringToName` (`KismetStringLibrary.Conv_IntToString` `Floor to Go To`)))
            (`|ExecutionSequence`
              (:`then_0`
                (break))
              (:`then_1`
                (set `self.targetFloorRef` _array_element_2)
                (set `self.targetFloor` `Floor to Go To`)
                (set `self.isMoving` true)
                (`self.Move Down`)))))))))

(event `self.ReceiveActorBeginOverlap`
  (params (OtherActor :type "Actor Object Reference")))

(event `self.ReceiveTick`
  (params (DeltaSeconds :type "Float (single-precision)")))

(event `Move Up`
  (if (<= (`self.GetDistanceTo` (`self.targetFloorRef`)) 6.0)
    (set `self.currentFloorRef` (`self.targetFloorRef`))
    (set `self.currentFloor` (`self.targetFloor`))
    (set `self.targetFloorRef` null)
    (`KismetSystemLibrary.Delay` 0.5)
    (set `self.isMoving` false)
    (else
      (`self.K2_SetActorLocation` (`KismetMathLibrary.MakeVector` (.x (`self.K2_GetActorLocation`)) (.y (`self.K2_GetActorLocation`)) (+ (.z (`self.K2_GetActorLocation`)) (`self.currentSpeed`))) true)
      (if (<= (`self.GetDistanceTo` (`self.currentFloorRef`)) 500.0)
        (set `self.currentSpeed` (+ (`self.currentSpeed`) 1.0))
        (`KismetSystemLibrary.Delay` 0.01)
        (`self.Move Up`)
        (elif (<= (`self.GetDistanceTo` (`self.targetFloorRef`)) 500.0)
          (set `self.currentSpeed` (- (`self.currentSpeed`) 1.0))
          (`KismetSystemLibrary.Delay` 0.01)
          (`self.Move Up`)
          (else
            (`KismetSystemLibrary.Delay` 0.01)
            (`self.Move Up`)))))))

(event `Move Down`
  (if (<= (`self.GetDistanceTo` (`self.targetFloorRef`)) 6.0)
    (set `self.currentFloorRef` (`self.targetFloorRef`))
    (set `self.currentFloor` (`self.targetFloor`))
    (set `self.targetFloorRef` null)
    (`KismetSystemLibrary.Delay` 0.5)
    (set `self.isMoving` false)
    (else
      (`self.K2_SetActorLocation` (`KismetMathLibrary.MakeVector` (.x (`self.K2_GetActorLocation`)) (.y (`self.K2_GetActorLocation`)) (- (.z (`self.K2_GetActorLocation`)) (`self.currentSpeed`))) true)
      (if (<= (`self.GetDistanceTo` (`self.currentFloorRef`)) 500.0)
        (set `self.currentSpeed` (+ (`self.currentSpeed`) 1.0))
        (`KismetSystemLibrary.Delay` 0.01)
        (`self.Move Down`)
        (elif (<= (`self.GetDistanceTo` (`self.targetFloorRef`)) 500.0)
          (set `self.currentSpeed` (- (`self.currentSpeed`) 1.0))
          (`KismetSystemLibrary.Delay` 0.01)
          (`self.Move Down`)
          (else
            (`KismetSystemLibrary.Delay` 0.01)
            (`self.Move Down`)))))))

(fn `UserConstructionScript`)