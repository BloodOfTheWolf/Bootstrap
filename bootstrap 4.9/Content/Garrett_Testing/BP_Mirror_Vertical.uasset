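; Laser puzzle mirror that tilts vertically through three pitch states and emits a reflected beam from a BP_Lazer child actor.
; The beam starts hidden and shows while its detector is struck by another visible laser, hiding once no lasers overlap.
; RotateUp and RotateDown step the pivot and beam, then re-project it.
; Projection uses a multi-object line trace to stretch the beam to the first mirror detector or Wall-tagged actor.
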(event `self.ReceiveBeginPlay`
  (`|ExecutionSequence`
    (:`then_0`
      ;[1 1 1] Enable input events to be allowed in this actor
      (`self.EnableInput` (`GameplayStatics.GetPlayerController` 0)))
    (:`then_1`
      ;[1 1 1] Create an initial reference to be used in the future
      (bind _asthird_person_character_1 (cast `/Game/ThirdPersonBP/Blueprints/ThirdPersonCharacter1` (`GameplayStatics.GetPlayerCharacter` 0)))
      (set `self.thirdPersonCharRef` _asthird_person_character_1))
    (:`then_2`
      ;[1 1 1] Create Lazer Ref
      (bind _asbp_lazer (cast `/Game/Garrett_Testing/BP_Lazer` (`ChildActorComponent.ChildActor` (`self.LazerActor`))))
      (set `self.myLazerRef` _asbp_lazer))
    (:`then_3`
      (`KismetSystemLibrary.Delay` 0.2)
      (switch `int` (`self.rotateState`)
        (:`1`
          (`self.UnconditionalRotateDown`))
        (:`2`
          _)
        (:`3`
          (`self.UnconditionalRotateUp`)))
      (`self.Project Lazer Path`))
    (:`then_4`
      ;[1 1 1] Hide Lazer Initially
      (`SceneComponent.SetVisibility` (`/Game/Garrett_Testing/BP_Lazer.LazerMesh` (`self.myLazerRef`)) false false))))

(event `Project Lazer Path`
  (bind _lazeractor (`self.LazerActor`))
  (bind _returnvalue (`SceneComponent.K2_GetComponentLocation` _lazeractor))
  (bind _outhits (`KismetSystemLibrary.LineTraceMultiForObjects` _returnvalue (+ (* (`SceneComponent.GetForwardVector` _lazeractor) 50000.0) _returnvalue) (`|MakeArray` "ObjectTypeQuery1" "ObjectTypeQuery2" :!type "EObjectTypeQuery Enum")))
  (for _array_element _outhits :!label _label
    (bind (_bblockinghit _binitialoverlap _time _location _impactpoint _normal _impactnormal _physmat _hitactor _hitcomponent) (`GameplayStatics.BreakHitResult` _array_element))
    (if (`KismetSystemLibrary.IsValid` _hitactor)
      (if (or (`KismetMathLibrary.ClassIsChildOf` (`GameplayStatics.GetObjectClass` _hitactor) "/Game/Garrett_Testing/BP_MirrorHorizontal.BP_MirrorHorizontal_C") (`KismetMathLibrary.ClassIsChildOf` (`GameplayStatics.GetObjectClass` _hitactor) "BP_Mirror_Vertical_C"))
        (if (`ActorComponent.ComponentHasTag` _hitcomponent "Detector")
          (`self.Break Loop`)
          (bind _output_get (set `self.destinationLocation` _impactpoint :!label _label_2))
          (`/Game/Garrett_Testing/BP_Lazer.ScaleAlongPath` (`self.myLazerRef`) _output_get))
        (elif (`self.ActorHasTag` _hitactor "Wall")
          (`self.Break Loop`)
          (goto _label_2))))))

(event `Break Loop`
  (goto _label :!via `Break`))

(event `self.LazerDetector.OnComponentBeginOverlap`
  (params (OtherActor :type "Actor Object Reference") (OtherComp :type "PrimitiveComponent Object Reference") (OtherBodyIndex :type Integer) (bFromSweep :type Boolean) (SweepResult :type "HitResult Structure (by ref)"))
  ;[1 1 1] Checks in the overlapped actor is a lazer, if so reveal this lazer
  (if (`KismetMathLibrary.ClassIsChildOf` (`GameplayStatics.GetObjectClass` OtherActor) "/Game/Garrett_Testing/BP_Lazer.BP_Lazer_C")
    (bind _asbp_lazer (cast `/Game/Garrett_Testing/BP_Lazer` OtherActor))
    (if (`SceneComponent.IsVisible` (`/Game/Garrett_Testing/BP_Lazer.LazerMesh` _asbp_lazer))
      (`SceneComponent.SetVisibility` (`/Game/Garrett_Testing/BP_Lazer.LazerMesh` (`self.myLazerRef`)) true true)
      (`KismetSystemLibrary.PrintString` "Overlapped"))))

(event `self.LazerDetector.OnComponentEndOverlap`
  (params (OtherActor :type "Actor Object Reference") (OtherComp :type "PrimitiveComponent Object Reference") (OtherBodyIndex :type Integer))
  ;[1 1 1] Hide the lazer when its no longer overlapped
  (if (`KismetMathLibrary.ClassIsChildOf` (`GameplayStatics.GetObjectClass` OtherActor) "/Game/Garrett_Testing/BP_Lazer.BP_Lazer_C")
    (if (not (`KismetSystemLibrary.IsValid` (`KismetArrayLibrary.Array_Get` (`PrimitiveComponent.GetOverlappingActors` (`self.LazerDetector`) "/Game/Garrett_Testing/BP_Lazer.BP_Lazer_C"))))
      (`SceneComponent.SetVisibility` (`/Game/Garrett_Testing/BP_Lazer.LazerMesh` (`self.myLazerRef`)) false true))))

(fn `DisableLazer`
  (`self.K2_DestroyActor` (`self.myLazer`))
  (`KismetSystemLibrary.PrintString` "destroyed"))

(fn `EnableLazer`
  ;[1 1 1] Spawn lazer with publicly set sizing, then immediately create a reference variable
  (bind _returnvalue (`|SpawnActorFromClass` "/Game/Garrett_Testing/BP_Lazer.BP_Lazer_C" (`SceneComponent.K2_GetComponentToWorld` (`self.LazerRefPoint`)) "AlwaysSpawn" "OverrideRootScale"))
  (set `self.myLazer` _returnvalue))

(fn `RotateDown`
  (bind _mirrorrotationpivot (`self.MirrorRotationPivot`))
  (if (> (`self.rotateState`) 1)
    (`|ExecutionSequence`
      (:`then_0`
        (`SceneComponent.K2_SetWorldLocationAndRotation` (`self.MirrorRotationPivot`) (`SceneComponent.K2_GetComponentLocation` _mirrorrotationpivot) (`KismetMathLibrary.MakeRotator` (.roll (`SceneComponent.K2_GetComponentRotation` _mirrorrotationpivot)) (- (.pitch (`SceneComponent.K2_GetComponentRotation` _mirrorrotationpivot)) (`self.rotateAmount`)) (.yaw (`SceneComponent.K2_GetComponentRotation` _mirrorrotationpivot))) false false))
      (:`then_1`
        (`SceneComponent.K2_SetWorldRotation` (`self.LazerActor`) (`KismetMathLibrary.MakeRotator` (.roll (`SceneComponent.K2_GetComponentRotation` (`self.LazerActor`))) (- (.pitch (`SceneComponent.K2_GetComponentRotation` (`self.LazerActor`))) 15.0) (.yaw (`SceneComponent.K2_GetComponentRotation` (`self.LazerActor`)))) false false))
      (:`then_2`
        (set `self.rotateState` (- (`self.rotateState`) 1))
        (`/Game/Garrett_Testing/BP_Lazer.ResetSize` (`self.myLazerRef`))
        (`self.Project Lazer Path`)))))

(fn `RotateUp`
  (bind _mirrorrotationpivot (`self.MirrorRotationPivot`))
  (if (< (`self.rotateState`) 3)
    (`|ExecutionSequence`
      (:`then_0`
        (`SceneComponent.K2_SetWorldLocationAndRotation` (`self.MirrorRotationPivot`) (`SceneComponent.K2_GetComponentLocation` _mirrorrotationpivot) (`KismetMathLibrary.MakeRotator` (.roll (`SceneComponent.K2_GetComponentRotation` _mirrorrotationpivot)) (+ (.pitch (`SceneComponent.K2_GetComponentRotation` _mirrorrotationpivot)) (`self.rotateAmount`)) (.yaw (`SceneComponent.K2_GetComponentRotation` _mirrorrotationpivot))) false false))
      (:`then_1`
        (`SceneComponent.K2_SetWorldRotation` (`self.LazerActor`) (`KismetMathLibrary.MakeRotator` (.roll (`SceneComponent.K2_GetComponentRotation` (`self.LazerActor`))) (+ (.pitch (`SceneComponent.K2_GetComponentRotation` (`self.LazerActor`))) 15.0) (.yaw (`SceneComponent.K2_GetComponentRotation` (`self.LazerActor`)))) false false))
      (:`then_2`
        (set `self.rotateState` (+ (`self.rotateState`) 1))
        (`/Game/Garrett_Testing/BP_Lazer.ResetSize` (`self.myLazerRef`))
        (`self.Project Lazer Path`)))))

(fn `UnconditionalRotateDown`
  (bind _mirrorrotationpivot (`self.MirrorRotationPivot`))
  (`|ExecutionSequence`
    (:`then_0`
      (`SceneComponent.K2_SetWorldLocationAndRotation` (`self.MirrorRotationPivot`) (`SceneComponent.K2_GetComponentLocation` _mirrorrotationpivot) (`KismetMathLibrary.MakeRotator` (.roll (`SceneComponent.K2_GetComponentRotation` _mirrorrotationpivot)) (- (.pitch (`SceneComponent.K2_GetComponentRotation` _mirrorrotationpivot)) (`self.rotateAmount`)) (.yaw (`SceneComponent.K2_GetComponentRotation` _mirrorrotationpivot))) false false))
    (:`then_1`
      (`SceneComponent.K2_SetWorldRotation` (`self.LazerActor`) (`KismetMathLibrary.MakeRotator` (.roll (`SceneComponent.K2_GetComponentRotation` (`self.LazerActor`))) (- (.pitch (`SceneComponent.K2_GetComponentRotation` (`self.LazerActor`))) 15.0) (.yaw (`SceneComponent.K2_GetComponentRotation` (`self.LazerActor`)))) false false))
    (:`then_2`
      (return))))

(fn `UnconditionalRotateUp`
  (bind _mirrorrotationpivot (`self.MirrorRotationPivot`))
  (`|ExecutionSequence`
    (:`then_0`
      (`SceneComponent.K2_SetWorldLocationAndRotation` (`self.MirrorRotationPivot`) (`SceneComponent.K2_GetComponentLocation` _mirrorrotationpivot) (`KismetMathLibrary.MakeRotator` (.roll (`SceneComponent.K2_GetComponentRotation` _mirrorrotationpivot)) (+ (.pitch (`SceneComponent.K2_GetComponentRotation` _mirrorrotationpivot)) (`self.rotateAmount`)) (.yaw (`SceneComponent.K2_GetComponentRotation` _mirrorrotationpivot))) false false))
    (:`then_1`
      (`SceneComponent.K2_SetWorldRotation` (`self.LazerActor`) (`KismetMathLibrary.MakeRotator` (.roll (`SceneComponent.K2_GetComponentRotation` (`self.LazerActor`))) (+ (.pitch (`SceneComponent.K2_GetComponentRotation` (`self.LazerActor`))) 15.0) (.yaw (`SceneComponent.K2_GetComponentRotation` (`self.LazerActor`)))) false false))
    (:`then_2`
      (return))))

(fn `UserConstructionScript`)