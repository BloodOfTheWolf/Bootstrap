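; Curtain actor that swaps the material on its Cube according to whether the player's camera is facing it.
; Each Tick compares the dot product of the camera's forward vector and its direction to the Cube against the character's Curtains threshold.
; It applies Mat1 above the threshold and Mat2 otherwise.
; Overlap-named events toggle a Checking flag, but nothing reads it, so the check always runs.
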(event `ReceiveActorBeginOverlap_Copy`
  (params (OtherActor :type "Actor Object Reference"))
  (set `self.Checking` true))

(event `self.ReceiveActorEndOverlap`
  (params (OtherActor :type "Actor Object Reference"))
  (set `self.Checking` false))

(event `self.ReceiveTick`
  (params (DeltaSeconds :type "Float (single-precision)"))
  (bind _cube (`self.Cube`))
  (`PrimitiveComponent.SetMaterial` _cube 0 (`self.mat1`))
  (if true
    (bind _asthird_person_character_1 (cast `/Game/ThirdPersonBP/Blueprints/ThirdPersonCharacter1` (`GameplayStatics.GetPlayerCharacter` 0)))
    (bind _fp_camera (`/Game/ThirdPersonBP/Blueprints/ThirdPersonCharacter1.FP_camera` _asthird_person_character_1))
    (if (> (`KismetMathLibrary.Dot_VectorVector` (`KismetMathLibrary.Normal` (- (`SceneComponent.K2_GetComponentLocation` _cube) (`SceneComponent.K2_GetComponentLocation` _fp_camera))) (`SceneComponent.GetForwardVector` _fp_camera)) (`/Game/ThirdPersonBP/Blueprints/ThirdPersonCharacter1.curtains` _asthird_person_character_1))
      (`PrimitiveComponent.SetMaterial` _cube 0 (`self.mat1`))
      (else
        (`PrimitiveComponent.SetMaterial` _cube 0 (`self.mat2`))))))

(fn `UserConstructionScript`)