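; Animated gate door actor that, on TriggerAnim, plays a mechanical opening sequence of panels, plug, locking rods and two doors.
; Its trigger volume enables player input and toggles prompt text on overlap; TriggerAnim has no caller in this graph.
; BeginPlay caches starting transforms, which timelines offset, chained through Update pins and staggered with Sequence and Delay nodes.
; The sequence also toggles steam and inset lights and later toggles rod visibility.
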(event `self.Trigger.OnComponentBeginOverlap`
  (params (OtherActor :type "Actor Object Reference") (OtherComp :type "PrimitiveComponent Object Reference") (OtherBodyIndex :type Integer) (bFromSweep :type Boolean) (SweepResult :type "HitResult Structure (by ref)"))
  ;[0.7919 1 0.8779] Input Range
  (`self.EnableInput` (`GameplayStatics.GetPlayerController` 0))
  (`SceneComponent.ToggleVisibility` (`self.PromptText`) false :!label _label))

(event `self.ReceiveBeginPlay`
  (bind _plugcap (`self.PlugCap`))
  ;[0.4202 0.5651 1] Glass
  (set `self.GlassStart` (`SceneComponent.RelativeLocation` (`self.GlassPanel`)))
  ;[0.5115 1 0.8136] GlassFrame
  (set `self.GlassFrameStart` (`SceneComponent.RelativeLocation` (`self.GlassFrame`)))
  ;[1 1 1] Initialize
  (set `self.PlugCapStart` (`SceneComponent.RelativeLocation` _plugcap))
  (set `self.PlugRot` (`SceneComponent.RelativeRotation` _plugcap))
  (set `self.DoorPlugStart` (`SceneComponent.RelativeLocation` (`self.DoorPlug`)))
  (set `self.TopRodStart` (`SceneComponent.RelativeLocation` (`self.RodTop`)))
  (set `self.BotRodStart` (`SceneComponent.RelativeLocation` (`self.RodBot`)))
  (set `self.MidRodStart` (`SceneComponent.RelativeLocation` (`self.RodMid`)))
  (set `self.LeftDoorStart` (`SceneComponent.RelativeLocation` (`self.LeftDoor`)))
  (set `self.RightDoorStart` (`SceneComponent.RelativeLocation` (`self.RightDoor`)))
  (set `self.FrameBackStart` (`SceneComponent.RelativeLocation` (`self.FrameBack`)))
  (set `self.PanelBackStart` (`SceneComponent.RelativeLocation` (`self.PanelBack`))))

(event `self.Trigger.OnComponentEndOverlap`
  (params (OtherActor :type "Actor Object Reference") (OtherComp :type "PrimitiveComponent Object Reference") (OtherBodyIndex :type Integer))
  ;[0.7919 1 0.8779] Input Range
  (`self.DisableInput` (`GameplayStatics.GetPlayerController` 0))
  (goto _label))

(event `Key|F`
  (params (Key :type "Key Structure" :default "AnyKey"))
  ;[1 0.9785 0.4785] Doors
)

(event `Key|F`
  (params (Key :type "Key Structure" :default "AnyKey"))
  ;[0.9365 0.6394 1] CenterCap
)

(event `Key|F`
  (params (Key :type "Key Structure" :default "AnyKey"))
  ;[0.5115 1 0.8136] GlassFrame
)

(event `Key|F`
  (params (Key :type "Key Structure" :default "AnyKey"))
  ;[1 0.9785 0.4785] Doors
)

(event `TriggerAnim`
  (bind (_plugrot_roll _plugrot_pitch _plugrot_yaw) (`KismetMathLibrary.BreakRotator` (`self.PlugRot`)))
  (bind (_direction _paneldown) (`Timeline|PanelBackMove`)
    (:`Update`
      (`SceneComponent.K2_SetRelativeLocation` (`self.PanelBack`) (+ _paneldown (`self.PanelBackStart`)) false false)
      (bind (_direction_2 _paneldown_2) (`Timeline|FrameBackMove`)
        (:`Update`
          (`SceneComponent.K2_SetRelativeLocation` (`self.FrameBack`) (+ _paneldown_2 (`self.FrameBackStart`)) false false)
          (`|ExecutionSequence`
            (:`then_0`
              ;[0.4202 0.5651 1] Glass
              (bind (_direction_3 _paneldown_3) (`Timeline|PanelDown`)
                (:`Update`
                  (`SceneComponent.K2_SetRelativeLocation` (`self.GlassPanel`) (+ _paneldown_3 (`self.GlassStart`)) false false)
                  ;[1 0.2597 0.2788] RotPlugCap
                  (bind (_direction_4 _rotate) (`Timeline|PlugCapRot`)
                    (:`Update`
                      (`SceneComponent.K2_SetRelativeRotation` (`self.PlugCap`) (`KismetMathLibrary.MakeRotator` (+ _rotate _plugrot_roll) 0.0 _plugrot_yaw) false false))))))
            (:`then_1`
              ;[0.5115 1 0.8136] GlassFrame
              (bind (_direction_5 _paneldown_4) (`Timeline|FrameDown`)
                (:`Update`
                  (`SceneComponent.K2_SetRelativeLocation` (`self.GlassFrame`) (+ _paneldown_4 (`self.GlassFrameStart`)) false false)
                  ;[0.9365 0.6394 1] CenterCap
                  (bind (_direction_6 _plugin) (`Timeline|PlugCapMove`)
                    (:`Update`
                      (`SceneComponent.K2_SetRelativeLocation` (`self.PlugCap`) (+ _plugin (`self.PlugCapStart`)) false false)
                      (`ActorComponent.ToggleActive` (`self.GrateSteam`))
                      (if false
                        (`KismetSystemLibrary.Delay` (`KismetMathLibrary.RandomFloatInRange` 0.01 0.35))
                        (else
                          (`KismetSystemLibrary.Delay` (`KismetMathLibrary.RandomFloatInRange` 1.0 2.0))))
                      (`SceneComponent.ToggleVisibility` (`self.InsetLightBot`) false)
                      (`SceneComponent.ToggleVisibility` (`self.InsetLightTop`) false))))))
            (:`then_2`
              (`KismetSystemLibrary.Delay` 2.0)
              (bind (_direction_7 _plugin_2) (`Timeline|DoorPlugOut`)
                (:`Update`
                  (`SceneComponent.K2_SetRelativeLocation` (`self.DoorPlug`) (+ _plugin_2 (`self.DoorPlugStart`)) false false))))
            (:`then_3`
              ;[1 0.9785 0.4785] Doors
              (`KismetSystemLibrary.Delay` 13.0)
              (bind (_direction_8 _plugin_3) (`Timeline|Timeline_1`)
                (:`Update`
                  (`SceneComponent.K2_SetRelativeLocation` (`self.RightDoor`) (+ _plugin_3 (`self.RightDoorStart`)) false false))))
            (:`then_4`
              (`KismetSystemLibrary.Delay` 13.0)
              (bind (_direction_9 _plugin_4) (`Timeline|Timeline_0`)
                (:`Update`
                  (`SceneComponent.K2_SetRelativeLocation` (`self.LeftDoor`) (+ _plugin_4 (`self.LeftDoorStart`)) false false))))
            (:`then_6`
              (`|ExecutionSequence`
                (:`then_0`
                  ;[1 0.4705 0.5665] Rods
                  (`KismetSystemLibrary.Delay` 5.0)
                  (bind (_direction_10 _plugin_5) (`Timeline|RodMoveTop`)
                    (:`Update`
                      (`SceneComponent.K2_SetRelativeLocation` (`self.RodTop`) (+ _plugin_5 (`self.TopRodStart`)) false false))))
                (:`then_1`
                  (`KismetSystemLibrary.Delay` 6.5)
                  (bind (_direction_11 _plugin_6) (`Timeline|RodMoveMid`)
                    (:`Update`
                      (`SceneComponent.K2_SetRelativeLocation` (`self.RodMid`) (+ _plugin_6 (`self.MidRodStart`)) false false)
                      (`KismetSystemLibrary.Delay` 7.0)
                      (`SceneComponent.ToggleVisibility` (`self.RodMid`) false)
                      (`SceneComponent.ToggleVisibility` (`self.RodBot`) false)
                      (`SceneComponent.ToggleVisibility` (`self.RodTop`) false))))
                (:`then_2`
                  (`KismetSystemLibrary.Delay` 8.0)
                  (bind (_direction_12 _plugin_7) (`Timeline|RodMoveBot`)
                    (:`Update`
                      (`SceneComponent.K2_SetRelativeLocation` (`self.RodBot`) (+ _plugin_7 (`self.BotRodStart`)) false false))))))))))))

(event `Key|F`
  (params (Key :type "Key Structure" :default "AnyKey"))
  ;[1 0.4705 0.5665] Rods
)

(event `Key|F`
  (params (Key :type "Key Structure" :default "AnyKey"))
  ;[1 0.4705 0.5665] Rods
)

(event `Key|F`
  (params (Key :type "Key Structure" :default "AnyKey"))
  ;[1 0.4705 0.5665] Rods
)

(fn `UserConstructionScript`)