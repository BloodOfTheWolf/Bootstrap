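; Floating multi-line text actor that pops up as a camera-facing sign with a backing cube and point light.
; Overlap by ThirdPersonCharacter1 spawns zero-scale text components, stacked vertically from TextLines, on every entry without clearing old ones.
; TextVisible and TextHidden toggle TextActive.
; Each tick, text turns toward the camera and grows while active or shrinks otherwise, driving cube scale and light intensity.
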(event `TextVisible`
  (set `self.TextActive` true))

(event `TextHidden`
  (set `self.TextActive` false))

(event `self.ReceiveActorBeginOverlap`
  (params (OtherActor :type "Actor Object Reference"))
  (if (`KismetMathLibrary.ClassIsChildOf` (`GameplayStatics.GetObjectClass` OtherActor) "/Game/ThirdPersonBP/Blueprints/ThirdPersonCharacter1.ThirdPersonCharacter1_C")
    ;[1 1 1] For Each Line of Text in the Object, Create a Text Render Object Using Each Line and Place Them a Set Distance Away From Each Other
    (for _index (range (`self.AmountOfLines`))
      (bind _item (`KismetArrayLibrary.Array_Get` (`self.TextLines`) _index))
      (if (> (`KismetStringLibrary.Len` _item) 0)
        (bind _returnvalue (`AddComponent|Text Render Component_12` :`RelativeTransform` (`KismetMathLibrary.MakeTransform` (`KismetMathLibrary.MakeVector` 10.0 0.0 (+ (+ (* _index -20.0) (* (`self.AmountOfLines`) 5.0)) 20.0)) (struct) (0.0 0.0 0.0))))
        (`PrimitiveComponent.SetMaterial` _returnvalue 0 "/Game/Materials/KevinMats/KevinTextMaterial.KevinTextMaterial")
        (`PrimitiveComponent.SetCastShadow` _returnvalue false)
        (`TextRenderComponent.SetHorizontalAlignment` _returnvalue "EHTA_Center")
        (`TextRenderComponent.K2_SetText` _returnvalue (`KismetTextLibrary.Conv_StringToText` _item))
        (`KismetArrayLibrary.Array_Add` (`self.TextRenderComponents`) _returnvalue)))))

(event `self.ReceiveTick`
  (params (DeltaSeconds :type "Float (single-precision)"))
  (for _array_element (`self.TextRenderComponents`)
    (if (`self.TextActive`)
      (bind _returnvalue (`KismetMathLibrary.FindLookAtRotation` (`SceneComponent.K2_GetComponentLocation` _array_element) (`self.K2_GetActorLocation` (`GameplayStatics.GetPlayerCameraManager` 0))))
      (`SceneComponent.K2_SetWorldRotation` _array_element _returnvalue false false)
      (`SceneComponent.K2_SetWorldRotation` (`self.Cube`) (`KismetMathLibrary.RInterpTo` (`SceneComponent.K2_GetComponentRotation` _array_element) _returnvalue (`GameplayStatics.GetWorldDeltaSeconds`) 4.0) false false)
      (bind _returnvalue_2 (`SceneComponent.K2_GetComponentScale` _array_element))
      (if (not (== _returnvalue_2 (1.0 1.0 1.0) :`ErrorTolerance` 0.0001))
        (`SceneComponent.SetWorldScale3D` _array_element (+ _returnvalue_2 (0.05 0.05 0.05)))
        (bind _x (.x (`SceneComponent.K2_GetComponentScale` _array_element)))
        (bind _z (.z (`SceneComponent.K2_GetComponentScale` _array_element)))
        (bind _returnvalue_3 (+ _x _x))
        (`SceneComponent.SetWorldScale3D` (`self.Cube`) (`KismetMathLibrary.MakeVector` 0.0 (* _returnvalue_3 1.5) _returnvalue_3))
        (`LightComponent.SetIntensity` (`self.PointLight`) (* _z 200.0)))
      (else
        (bind _returnvalue_4 (`SceneComponent.K2_GetComponentScale` _array_element))
        (if (not (== _returnvalue_4 (0.0 0.0 0.0) :`ErrorTolerance` 0.0001))
          (`SceneComponent.SetWorldScale3D` _array_element (- _returnvalue_4 (0.05 0.05 0.05)))
          (bind _returnvalue_5 (/ _x 2.0))
          (`SceneComponent.SetWorldScale3D` (`self.Cube`) (`KismetMathLibrary.MakeVector` 0.0 (* _returnvalue_5 1.5) _returnvalue_5))
          (`LightComponent.SetIntensity` (`self.PointLight`) (/ _z 200.0)))))))

(fn `UserConstructionScript`
  (bind _returnvalue (`KismetArrayLibrary.Array_Length` (`self.TextLines`)))
  ;[1 1 1] Set the Amount of Lines in the Object and Set the Largest Size by Character Length
  (set `self.AmountOfLines` _returnvalue)
  (for _index (range _returnvalue)
    (set `self.MostLines` (`KismetMathLibrary.Max` (`KismetStringLibrary.Len` (`KismetArrayLibrary.Array_Get` (`self.TextLines`) _index)) (`self.MostLines`)))))