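; Prompt arrow Blueprint that animates a repeated slide toward a target point, apparently as a directional cue.
; On BeginPlay, it moves Mover to Target's relative location over Duration, pauses briefly, snaps back and repeats until the tally equals MaxTally.
; The ArrowPlay event re-enters the same loop without resetting the tally.
; The Construction Script applies the Color material to the arrow.
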(event `self.ReceiveBeginPlay`
  (`|ExecutionSequence`
    (:`then_1`
      (set `self.Arrow Start` (`SceneComponent.RelativeLocation` (`self.Mover`)))
      (set `self.TargetLocation` (`SceneComponent.RelativeLocation` (`self.Target`)))
      (set `self.tally` 0)
      (`KismetSystemLibrary.MoveComponentTo` (`self.Mover`) (`self.TargetLocation`) (struct) false false (`self.Duration`) :!label _label)
      (`KismetSystemLibrary.Delay` 0.3)
      (`KismetSystemLibrary.MoveComponentTo` (`self.Mover`) (`self.Arrow Start`) (struct) false false 0.0)
      (set `self.newPos` (`SceneComponent.RelativeLocation` (`self.Mover`)))
      (if (== (`self.Arrow Start`) (`self.newPos`))
        (set `self.tally` (+ (`self.tally`) 1))
        (if (not (== (`self.tally`) (`self.Max Tally`)))
          (goto _label))))))

(event `ArrowPlay`
  (params (NewParam :type Boolean))
  (goto _label))

(fn `UserConstructionScript`
  (`PrimitiveComponent.SetMaterial` (`self.Arrow`) 0 (`self.Color`)))