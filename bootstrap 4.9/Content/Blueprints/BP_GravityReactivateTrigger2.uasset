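; Trigger volume that switches player gravity while the player overlaps it and the character's GlobalAntigrav flag is set.
; Each Tick polls the overlap via the Sphere's owner, then runs two sequenced checks on IsAntigrav.
; The first restores gravity and Walking, the second sets zero gravity and Flying.
; Because the second sees the first's change, every overlapping tick ends in antigrav.
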(event `self.ReceiveBeginPlay`)

(event `self.ReceiveActorBeginOverlap`
  (params (OtherActor :type "Actor Object Reference")))

(event `self.ReceiveTick`
  (params (DeltaSeconds :type "Float (single-precision)"))
  (bind _returnvalue (`GameplayStatics.GetPlayerCharacter` 0))
  (bind _returnvalue_2 (`self.IsOverlappingActor` (`ActorComponent.GetOwner` (`self.Sphere`)) _returnvalue))
  (bind _asthird_person_character_1 (cast `/Game/ThirdPersonBP/Blueprints/ThirdPersonCharacter1` (`GameplayStatics.GetPlayerCharacter` 0)))
  (if (`/Game/ThirdPersonBP/Blueprints/ThirdPersonCharacter1.GlobalAntigrav` _asthird_person_character_1)
    (`|ExecutionSequence`
      (:`then_0`
        (if _returnvalue_2
          (bind _isantigrav_ (`/Game/ThirdPersonBP/Blueprints/ThirdPersonCharacter1.IsAntigrav?` _asthird_person_character_1))
          (if _isantigrav_
            (bind _asthird_person_character_1_2 (cast `/Game/ThirdPersonBP/Blueprints/ThirdPersonCharacter1` _returnvalue))
            (if (`/Game/ThirdPersonBP/Blueprints/ThirdPersonCharacter1.IsAntigrav?` _asthird_person_character_1_2)
              (bind _charactermovement (`Character.CharacterMovement` _asthird_person_character_1_2))
              (set `CharacterMovementComponent.GravityScale` 1.0 _charactermovement)
              (`CharacterMovementComponent.SetMovementMode` _charactermovement "MOVE_Walking" 0)
              (set `/Game/ThirdPersonBP/Blueprints/ThirdPersonCharacter1.IsAntigrav?` false _asthird_person_character_1_2)))))
      (:`then_1`
        (if _returnvalue_2
          (if (not _isantigrav_)
            (bind _asthird_person_character_1_3 (cast `/Game/ThirdPersonBP/Blueprints/ThirdPersonCharacter1` _returnvalue))
            (if (not (`/Game/ThirdPersonBP/Blueprints/ThirdPersonCharacter1.IsAntigrav?` _asthird_person_character_1_3))
              (bind _charactermovement_2 (`Character.CharacterMovement` _asthird_person_character_1_3))
              (set `CharacterMovementComponent.GravityScale` 0.0 _charactermovement_2)
              (`CharacterMovementComponent.SetMovementMode` _charactermovement_2 "MOVE_Flying" 0)
              (set `/Game/ThirdPersonBP/Blueprints/ThirdPersonCharacter1.IsAntigrav?` true _asthird_person_character_1_3))))))))

(fn `UserConstructionScript`)