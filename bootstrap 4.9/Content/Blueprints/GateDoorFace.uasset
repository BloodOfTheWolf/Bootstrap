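; Front half of an animated gate door that opens when the player presses F inside its trigger, which enables input and toggles a prompt.
; F triggers the GateDoorBack tagged OtherDoor, plus delayed timelines that offset glass, frame, plug, rods and sliding doors from cached starting transforms.
; Timeline updates also chain cap motion, steam toggling and randomly delayed light flicker.
; An openGate event replays most of the sequence, omitting the rods.
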(event `self.Trigger.OnComponentBeginOverlap`
  (params (OtherActor :type "Actor Object Reference") (OtherComp :type "PrimitiveComponent Object Reference") (OtherBodyIndex :type Integer) (bFromSweep :type Boolean) (SweepResult :type "HitResult Structure (by ref)"))
  ;[0.7919 1 0.8779] Input Range
  (`self.EnableInput` (`GameplayStatics.GetPlayerController` 0))
  (`SceneComponent.ToggleVisibility` (`self.PromptText`) false :!label _label))

(event `self.ReceiveBeginPlay`
  (bind _plugcap (`self.PlugCap`))
  ;[1 1 1] Initialize
  (set `self.GlassStart` (`SceneComponent.RelativeLocation` (`self.GlassPanel`)))
  (set `self.GlassFrameStart` (`SceneComponent.RelativeLocation` (`self.GlassFrame`)))
  (set `self.PlugCapStart` (`SceneComponent.RelativeLocation` _plugcap))
  (set `self.PlugRot` (`SceneComponent.RelativeRotation` _plugcap))
  (set `self.DoorPlugStart` (`SceneComponent.RelativeLocation` (`self.DoorPlug`)))
  (set `self.TopRodStart` (`SceneComponent.RelativeLocation` (`self.RodTop`)))
  (set `self.BotRodStart` (`SceneComponent.RelativeLocation` (`self.RodBot`)))
  (set `self.MidRodStart` (`SceneComponent.RelativeLocation` (`self.RodMid`)))
  (set `self.LeftDoorStart` (`SceneComponent.RelativeLocation` (`self.LeftDoor`)))
  (set `self.RightDoorStart` (`SceneComponent.RelativeLocation` (`self.RightDoor`)))
  (set `self.TargetBackHalf` null))

(event `self.Trigger.OnComponentEndOverlap`
  (params (OtherActor :type "Actor Object Reference") (OtherComp :type "PrimitiveComponent Object Reference") (OtherBodyIndex :type Integer))
  ;[0.7919 1 0.8779] Input Range
  (`self.DisableInput` (`GameplayStatics.GetPlayerController` 0))
  (goto _label))

(event `Key|F`
  (params (Key :type "Key Structure" :default "AnyKey"))
  (bind (_plugrot_roll _plugrot_pitch _plugrot_yaw) (`KismetMathLibrary.BreakRotator` (`self.PlugRot`)))
  ;[1 0.8634 0.2916] Activate my Mate
  (:`Pressed`
    (bind _outactors (`GameplayStatics.GetAllActorsOfClass` "/Game/Blueprints/GateDoorBack.GateDoorBack_C" :!label _label_2))
    (for _array_element _outactors
      (if (!= (`self.otherDoor`) "None")
        (if (`self.ActorHasTag` _array_element (`self.otherDoor`))
          (`/Game/Blueprints/GateDoorBack.TriggerAnim` _array_element)
          ;[0.4202 0.5651 1] Glass
          (bind (_direction _paneldown) (`Timeline|PanelDown`)
            (:`Update`
              (`SceneComponent.K2_SetRelativeLocation` (`self.GlassPanel`) (+ _paneldown (`self.GlassStart`)) false false)
              ;[1 0.2597 0.2788] RotPlugCap
              (bind (_direction_2 _rotate) (`Timeline|PlugCapRot`)
                (:`Update`
                  (`SceneComponent.K2_SetRelativeRotation` (`self.PlugCap`) (`KismetMathLibrary.MakeRotator` (+ _rotate _plugrot_roll) 0.0 _plugrot_yaw) false false))))))))))

(event `openGate`
  (`|ExecutionSequence`
    (:`then_0`
      (goto _label_2))
    (:`then_1`
      ;[1 0.9785 0.4785] Doors
      (`KismetSystemLibrary.Delay` 11.0 :!label _label_3)
      (bind (_direction _doorstate) (`Timeline|DoorLeftSlide`)
        (:`Update`
          (`SceneComponent.K2_SetRelativeLocation` (`self.RightDoor`) (+ _doorstate (`self.RightDoorStart`)) false false))))
    (:`then_2`
      ;[0.5115 1 0.8136] GlassFrame
      (bind (_direction_2 _paneldown) (`Timeline|FrameDown` :!label _label_4)
        (:`Update`
          (`SceneComponent.K2_SetRelativeLocation` (`self.GlassFrame`) (+ _paneldown (`self.GlassFrameStart`)) false false)
          ;[0.9365 0.6394 1] CenterCap
          (bind (_direction_3 _plugin) (`Timeline|PlugCapMove`)
            (:`Update`
              (`SceneComponent.K2_SetRelativeLocation` (`self.PlugCap`) (+ _plugin (`self.PlugCapStart`)) false false)
              (`ActorComponent.ToggleActive` (`self.GrateSteam`))
              (set `self.randomFlickerValue` (`KismetMathLibrary.RandomInteger` 2))
              (if (== (`self.randomFlickerValue`) 0)
                (`KismetSystemLibrary.Delay` (`KismetMathLibrary.RandomFloatInRange` 0.01 0.35))
                (else
                  (`KismetSystemLibrary.Delay` (`KismetMathLibrary.RandomFloatInRange` 1.0 2.0))))
              (`SceneComponent.ToggleVisibility` (`self.InsetLightBot`) false)
              (`SceneComponent.ToggleVisibility` (`self.InsetLightTop`) false))))))
    (:`then_3`
      (`KismetSystemLibrary.Delay` 2.0 :!label _label_5)
      (bind (_direction_4 _plugin_2) (`Timeline|DoorPlugOut`)
        (:`Update`
          (`SceneComponent.K2_SetRelativeLocation` (`self.DoorPlug`) (+ _plugin_2 (`self.DoorPlugStart`)) false false))))
    (:`then_4`
      (`KismetSystemLibrary.Delay` 11.0 :!label _label_6)
      (bind (_direction_5 _doorstate_2) (`Timeline|DoorRightSlide`)
        (:`Update`
          (`SceneComponent.K2_SetRelativeLocation` (`self.LeftDoor`) (+ _doorstate_2 (`self.LeftDoorStart`)) false false)
          (`KismetSystemLibrary.Delay` 3.0)
          (if (`SceneComponent.IsVisible` (`self.PromptText`))
            (`SceneComponent.ToggleVisibility` (`self.PromptText`) false)))))))

(event `Key|F`
  (params (Key :type "Key Structure" :default "AnyKey"))
  ;[1 0.9785 0.4785] Doors
  (:`Pressed`
    (goto _label_3)))

(event `Key|F`
  (params (Key :type "Key Structure" :default "AnyKey"))
  ;[0.9365 0.6394 1] CenterCap
  (:`Pressed`
    (goto _label_5)))

(event `Key|F`
  (params (Key :type "Key Structure" :default "AnyKey"))
  (:`Pressed`
    (goto _label_6)))

(event `Key|F`
  (params (Key :type "Key Structure" :default "AnyKey"))
  ;[0.5115 1 0.8136] GlassFrame
  (:`Pressed`
    (goto _label_4)))

(event `Key|F`
  (params (Key :type "Key Structure" :default "AnyKey"))
  ;[1 0.4705 0.5665] Rods
  (:`Pressed`
    (`KismetSystemLibrary.Delay` 5.0)
    (bind (_direction _plugin) (`Timeline|RodMoveTop`)
      (:`Update`
        (`SceneComponent.K2_SetRelativeLocation` (`self.RodTop`) (+ _plugin (`self.TopRodStart`)) false false)))))

(event `Key|F`
  (params (Key :type "Key Structure" :default "AnyKey"))
  ;[1 0.4705 0.5665] Rods
  (:`Pressed`
    (`KismetSystemLibrary.Delay` 6.5)
    (bind (_direction _plugin) (`Timeline|RodMoveMid`)
      (:`Update`
        (`SceneComponent.K2_SetRelativeLocation` (`self.RodMid`) (+ _plugin (`self.MidRodStart`)) false false)
        (`KismetSystemLibrary.Delay` 7.0)
        (`SceneComponent.ToggleVisibility` (`self.RodMid`) false)
        (`SceneComponent.ToggleVisibility` (`self.RodBot`) false)
        (`SceneComponent.ToggleVisibility` (`self.RodTop`) false)))))

(event `Key|F`
  (params (Key :type "Key Structure" :default "AnyKey"))
  ;[1 0.4705 0.5665] Rods
  (:`Pressed`
    (`KismetSystemLibrary.Delay` 8.0)
    (bind (_direction _plugin) (`Timeline|RodMoveBot`)
      (:`Update`
        (`SceneComponent.K2_SetRelativeLocation` (`self.RodBot`) (+ _plugin (`self.BotRodStart`)) false false)))))

(fn `UserConstructionScript`)