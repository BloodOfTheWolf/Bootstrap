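; Multi-floor elevator that moves vertically between TargetPoints tagged with floor numbers, snapping to its starting floor on BeginPlay.
; A timeline swings the door open when the player character enters the trigger; a separate timeline event rotates the cabin's Center.
; GoToFloor closes the door, then picks up or down movement.
; Movement loops through per-frame Delay re-calls, easing speed near either floor, and reopens the door on arrival.
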(event `openEle`
  (bind (_doorrot_roll _doorrot_pitch _doorrot_yaw) (`KismetMathLibrary.BreakRotator` (`self.DoorRot`)))
  (bind (_direction _rotate) (`Timeline|Door Rotation` :!label _label)
    (:`Update`
      (`SceneComponent.K2_SetRelativeRotation` (`self.Door Pivot`) (`KismetMathLibrary.MakeRotator` 0.0 0.0 (+ _rotate _doorrot_yaw)) false false)
      (set `self.Open` true))))

(event `self.Trigger.OnComponentBeginOverlap`
  (params (OtherActor :type "Actor Object Reference") (OtherComp :type "PrimitiveComponent Object Reference") (OtherBodyIndex :type Integer) (bFromSweep :type Boolean) (SweepResult :type "HitResult Structure (by ref)"))
  (if (`KismetMathLibrary.ClassIsChildOf` (`GameplayStatics.GetObjectClass` OtherActor) "/Game/ThirdPersonBP/Blueprints/ThirdPersonCharacter1.ThirdPersonCharacter1_C")
    (goto _label)))

(event `closeEle`
  (goto _label :!via `Reverse`))

(event `180 Elevator`
  (bind (_elevator_pivot_roll _elevator_pivot_pitch _elevator_pivot_yaw) (`KismetMathLibrary.BreakRotator` (`self.Elevator Pivot`)))
  (bind (_direction _rotate) (`Timeline|Timeline_0`)
    (:`Update`
      (`SceneComponent.K2_SetRelativeRotation` (`self.Center`) (`KismetMathLibrary.MakeRotator` 0.0 0.0 (+ _rotate _elevator_pivot_yaw)) false false))))

(event `self.Trigger.OnComponentEndOverlap`
  (params (OtherActor :type "Actor Object Reference") (OtherComp :type "PrimitiveComponent Object Reference") (OtherBodyIndex :type Integer)))

(event `self.ReceiveBeginPlay`
  ;[1 1 1] Grab all floor target points and add them into an array
  (bind _outactors (`GameplayStatics.GetAllActorsOfClass` "/Script/Engine.TargetPoint"))
  (for _array_element _outactors
    (`KismetArrayLibrary.Array_Add` (`self.floorArray`) _array_element)
    (set `self.DoorRot` (`SceneComponent.RelativeRotation` (`self.Door Pivot`)))
    (set `self.Elevator Pivot` (`SceneComponent.RelativeRotation` (`self.Center`))))
  ;[1 1 1] Teleports the elevator to the starting floor designated by the 'startingFloor' var
  (for _array_element_2 (`self.floorArray`)
    (if (`self.ActorHasTag` _array_element_2 (`KismetStringLibrary.Conv_StringToName` (`KismetStringLibrary.Conv_IntToString` (`self.startingFloor`))))
      (`self.K2_SetActorLocation` (`self.K2_GetActorLocation` _array_element_2))
      (set `self.currentFloor` (`self.startingFloor`))
      (set `self.currentFloorRef` _array_element_2))))

(event `Go To Floor`
  (params (`Floor to Go To` :type Integer))
  (if (not (`self.isMoving`))
    (`self.closeEle`)
    (`KismetSystemLibrary.Delay` 2.5)
    (`/Engine/EditorBlueprintResources/StandardMacros.CompareInt` `Floor to Go To` (`self.currentFloor`)
      (:`>`
        (for _array_element (`self.floorArray`)
          (if (`self.ActorHasTag` _array_element (`KismetStringLibrary.Conv_StringToName` (`KismetStringLibrary.Conv_IntToString` `Floor to Go To`)))
            (`|ExecutionSequence`
              (:`then_0`
                (break))
              (:`then_1`
                (set `self.targetFloorRef` _array_element)
                (set `self.targetFloor` `Floor to Go To`)
                (set `self.isMoving` true)
                (`self.Move Up`))))))
      (:`<`
        (for _array_element_2 (`self.floorArray`)
          (if (`self.ActorHasTag` _array_element_2 (`KismetStringLibrary.Conv_StringToName` (`KismetStringLibrary.Conv_IntToString` `Floor to Go To`)))
            (`|ExecutionSequence`
              (:`then_0`
                (break))
              (:`then_1`
                (set `self.targetFloorRef` _array_element_2)
                (set `self.targetFloor` `Floor to Go To`)
                (set `self.isMoving` true)
                (`self.Move Down`)))))))))

(event `Move Up`
  (if (<= (`self.GetDistanceTo` (`self.targetFloorRef`)) (`self.errorRange`))
    (set `self.currentFloorRef` (`self.targetFloorRef`))
    (set `self.currentFloor` (`self.targetFloor`))
    (set `self.targetFloorRef` null)
    (`self.openEle`)
    (`KismetSystemLibrary.Delay` 0.5)
    (set `self.isMoving` false)
    (else
      (`self.K2_SetActorLocation` (`KismetMathLibrary.MakeVector` (.x (`self.K2_GetActorLocation`)) (.y (`self.K2_GetActorLocation`)) (+ (.z (`self.K2_GetActorLocation`)) (`self.currentSpeed`))) true)
      (if (<= (`self.GetDistanceTo` (`self.currentFloorRef`)) 500.0)
        (set `self.currentSpeed` (+ (`self.currentSpeed`) 1.0))
        (`KismetSystemLibrary.Delay` (stale `self.ReceiveTick` DeltaSeconds))
        (`self.Move Up`)
        (elif (<= (`self.GetDistanceTo` (`self.targetFloorRef`)) 500.0)
          (set `self.currentSpeed` (- (`self.currentSpeed`) 1.0))
          (`KismetSystemLibrary.Delay` (stale `self.ReceiveTick` DeltaSeconds))
          (`self.Move Up`)
          (else
            (`KismetSystemLibrary.Delay` (stale `self.ReceiveTick` DeltaSeconds))
            (`self.Move Up`)))))))

(event `self.ReceiveTick`
  (params (DeltaSeconds :type "Float (single-precision)")))

(event `Move Down`
  (if (<= (`self.GetDistanceTo` (`self.targetFloorRef`)) (`self.errorRange`))
    (set `self.currentFloorRef` (`self.targetFloorRef`))
    (set `self.currentFloor` (`self.targetFloor`))
    (set `self.targetFloorRef` null)
    (`self.openEle`)
    (`KismetSystemLibrary.Delay` 0.5)
    (set `self.isMoving` false)
    (else
      (`self.K2_SetActorLocation` (`KismetMathLibrary.MakeVector` (.x (`self.K2_GetActorLocation`)) (.y (`self.K2_GetActorLocation`)) (- (.z (`self.K2_GetActorLocation`)) (`self.currentSpeed`))) true)
      (if (<= (`self.GetDistanceTo` (`self.currentFloorRef`)) 500.0)
        (set `self.currentSpeed` (+ (`self.currentSpeed`) 1.0))
        (`KismetSystemLibrary.Delay` (stale `self.ReceiveTick` DeltaSeconds))
        (`self.Move Down`)
        (elif (<= (`self.GetDistanceTo` (`self.targetFloorRef`)) 500.0)
          (set `self.currentSpeed` (- (`self.currentSpeed`) 1.0))
          (`KismetSystemLibrary.Delay` (stale `self.ReceiveTick` DeltaSeconds))
          (`self.Move Down`)
          (else
            (`KismetSystemLibrary.Delay` (stale `self.ReceiveTick` DeltaSeconds))
            (`self.Move Down`)))))))

(fn `UserConstructionScript`)