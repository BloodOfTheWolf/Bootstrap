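; Configurable floor signage actor that shows its OuterCharge component when the player character comes near.
; The construction script applies exposed text, colors and materials to the floor label, number, description, inset and charge.
; Entering the trigger toggles the hidden charge visible after a randomly short or long delay, varying when it appears.
; Leaving the trigger hides the charge immediately if it is visible.
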(event OnComponentBeginOverlap(Trigger)
  (params (OtherActor :type Actor%20Object%20Reference) (OtherComp :type Primitive%20Component%20Object%20Reference) (OtherBodyIndex :type Integer) (bFromSweep :type Boolean) (SweepResult :type Hit%20Result%20Structure%20%28by%20ref%29))
  (if (Utilities|ClassIsChildOf (Utilities|GetClass OtherActor) "/Game/ThirdPersonBP/Blueprints/ThirdPersonCharacter1.ThirdPersonCharacter1_C")
    (if (not (Rendering|IsVisible (Variables|Default|GetOuterCharge)))
      (Variables|Default|SetrandomFlickerValue (Math|Random|RandomInteger 2))
      (if (== (Variables|Default|GetRandomFlickerValue) 0)
        (Utilities|FlowControl|Delay (Math|Random|RandomFloatinRange 0.01 0.35))
        (else
          (Utilities|FlowControl|Delay (Math|Random|RandomFloatinRange 1.0 2.0))))
      (Rendering|ToggleVisibility (Variables|Default|GetOuterCharge) false))))

(event OnComponentEndOverlap(Trigger)
  (params (OtherActor :type Actor%20Object%20Reference) (OtherComp :type Primitive%20Component%20Object%20Reference) (OtherBodyIndex :type Integer))
  (if (Utilities|ClassIsChildOf (Utilities|GetClass OtherActor) "/Game/ThirdPersonBP/Blueprints/ThirdPersonCharacter1.ThirdPersonCharacter1_C")
    (if (Rendering|IsVisible (Variables|Default|GetOuterCharge))
      (Rendering|ToggleVisibility (Variables|Default|GetOuterCharge) false))))

(fn ConstructionScript
  (Rendering|Components|TextRender|SetTextRenderColor (Variables|Default|GetFloor) (Math|Color|MakeColor (Variables|Default|Getblue) (Variables|Default|GetGreen) (Variables|Default|GetRed) 255))
  (Rendering|Components|TextRender|SetText (Variables|Default|GetNumText) (Variables|Default|GetNumber))
  (Rendering|Material|SetMaterial (Variables|Default|Getinset) 0 (Variables|Default|GetEmissiveMat))
  (Rendering|Material|SetMaterial (Variables|Default|GetOuterCharge) 0 (Variables|Default|GetCharge%20Color))
  (Rendering|Components|TextRender|SetText (Variables|Default|GetDescription) (Variables|Default|GetFloorDescription))
  (Rendering|Components|TextRender|SetTextRenderColor (Variables|Default|GetDescription) (Math|Color|MakeColor (Variables|Default|GetBlue2) (Variables|Default|GetGreen2) (Variables|Default|GetRed2) 255)))