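; Interactive screen actor whose frame moves and grows on an H key press while the player is inside its trigger volume.
; Overlap enables input and toggles a prompt; MoveFrame and Grow timelines offset the frame's starting location and scale in staggered order.
; A randomized delay then toggles the screen and spotlight, re-showing the screen if hidden.
; Leaving disables input, toggles the prompt, reverses both timelines and hides a visible screen and light.
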(event `self.ReceiveBeginPlay`
  (bind _frame (`self.frame`))
  ;[1 1 1] Initialize
  (set `self.frameStart` (`SceneComponent.RelativeLocation` _frame))
  (set `self.frameSize` (`SceneComponent.RelativeScale3D` _frame)))

(event `Key|H`
  (params (Key :type "Key Structure" :default "AnyKey"))
  ;[1 0.4562 0.9798] Action
  (:`Pressed`
    (`|ExecutionSequence`
      (:`then_0`
        (bind (_direction _paneldown) (`Timeline|MoveFrame` :!label _label)
          (:`Update`
            (`SceneComponent.K2_SetRelativeLocation` (`self.frame`) (+ _paneldown (`self.frameStart`)) false false))))
      (:`then_1`
        (`KismetSystemLibrary.Delay` 2.2)
        (bind (_direction_2 _inflate) (`Timeline|Grow` :!label _label_2)
          (:`Update`
            (`SceneComponent.SetRelativeScale3D` (`self.frame`) (+ _inflate (`self.frameSize`))))))
      (:`then_2`
        (`KismetSystemLibrary.Delay` 2.5)
        (set `self.randomFlickerValue` (`KismetMathLibrary.RandomInteger` 2))
        (if (== (`self.RandomFlickerValue`) 0)
          (`KismetSystemLibrary.Delay` (`KismetMathLibrary.RandomFloatInRange` 0.01 0.35))
          (else
            (`KismetSystemLibrary.Delay` (`KismetMathLibrary.RandomFloatInRange` 1.0 2.0))))
        (`SceneComponent.ToggleVisibility` (`self.Screen`) false)
        (`SceneComponent.ToggleVisibility` (`self.SpotLight`) false)
        (if (not (`SceneComponent.IsVisible` (`self.Screen`)))
          (`SceneComponent.ToggleVisibility` (`self.Screen`) false))))))

(event `self.Trigger.OnComponentBeginOverlap`
  (params (OtherActor :type "Actor Object Reference") (OtherComp :type "PrimitiveComponent Object Reference") (OtherBodyIndex :type Integer) (bFromSweep :type Boolean) (SweepResult :type "HitResult Structure (by ref)"))
  ;[0.7919 1 0.8779] Input Range
  (`self.EnableInput` (`GameplayStatics.GetPlayerController` 0))
  (`SceneComponent.ToggleVisibility` (`self.MorePrompt`) false :!label _label_3))

(event `self.Trigger.OnComponentEndOverlap`
  (params (OtherActor :type "Actor Object Reference") (OtherComp :type "PrimitiveComponent Object Reference") (OtherBodyIndex :type Integer))
  ;[0.7919 1 0.8779] Input Range
  (`|ExecutionSequence`
    (:`then_0`
      (`self.DisableInput` (`GameplayStatics.GetPlayerController` 0))
      (goto _label_3))
    (:`then_1`
      (goto _label :!via `Reverse`))
    (:`then_2`
      ;[1 1 1] Hide
      (if (`SceneComponent.IsVisible` (`self.Screen`))
        (`SceneComponent.ToggleVisibility` (`self.Screen`) false)
        (`SceneComponent.ToggleVisibility` (`self.SpotLight`) false)))
    (:`then_3`
      (goto _label_2 :!via `Reverse`))))

(fn `UserConstructionScript`)