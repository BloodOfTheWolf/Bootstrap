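; Interactive shutter actor that animates two valve handles and two panels when G is pressed inside its trigger volume.
; Trigger overlap enables and disables input, and G plays all timelines at once, offsetting parts from transforms cached on BeginPlay.
; Valve rotation updates also toggle each side's sparks after a delay plus a random short or long wait, creating flicker.
; The right valve's rotation is based on the left valve's starting rotation.
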(event `self.ReceiveBeginPlay`
  ;[0.6917 1 0.1727] Initialize
  (`|ExecutionSequence`
    (:`then_0`
      (set `self.StartPosVRight` (`SceneComponent.RelativeLocation` (`self.ValveRight`))))
    (:`then_1`
      (set `self.StartPosVLeft` (`SceneComponent.RelativeLocation` (`self.ValveLeft`))))
    (:`then_2`
      (set `self.StartPosPLeft` (`SceneComponent.RelativeLocation` (`self.PanelLeft`))))
    (:`then_3`
      (set `self.StartPosPRight` (`SceneComponent.RelativeLocation` (`self.PanelRight`))))
    (:`then_4`
      (set `self.StartRotVLeft` (`SceneComponent.RelativeRotation` (`self.ValveLeft`))))
    (:`then_5`
      (set `self.StartRotVRight` (`SceneComponent.RelativeRotation` (`self.ValveRight`))))))

(event `self.Trigger.OnComponentBeginOverlap`
  (params (OtherActor :type "Actor Object Reference") (OtherComp :type "PrimitiveComponent Object Reference") (OtherBodyIndex :type Integer) (bFromSweep :type Boolean) (SweepResult :type "HitResult Structure (by ref)"))
  ;[0.5403 0.6485 1] Input Range
  (`self.EnableInput` (`GameplayStatics.GetPlayerController` 0)))

(event `self.Trigger.OnComponentEndOverlap`
  (params (OtherActor :type "Actor Object Reference") (OtherComp :type "PrimitiveComponent Object Reference") (OtherBodyIndex :type Integer))
  ;[0.5403 0.6485 1] Input Range
  (`self.DisableInput` (`GameplayStatics.GetPlayerController` 0)))

(event `Key|G` :consume false
  (params (Key :type "Key Structure" :default "AnyKey"))
  (bind (_startrotvleft_roll _startrotvleft_pitch _startrotvleft_yaw) (`KismetMathLibrary.BreakRotator` (`self.StartRotVLeft`)))
  (bind (_startrotvleft_roll_2 _startrotvleft_pitch_2 _startrotvleft_yaw_2) (`KismetMathLibrary.BreakRotator` (`self.StartRotVLeft`)))
  ;[1 0.3723 0.9932] Start
  (:`Pressed`
    (`|ExecutionSequence`
      (:`then_0`
        ;[0.1199 1 0.9905] ValveHandles
        (`|ExecutionSequence`
          (:`then_0`
            (bind (_direction _plugin) (`Timeline|LeftValveIn`)
              (:`Update`
                (`SceneComponent.K2_SetRelativeLocation` (`self.ValveLeft`) (+ _plugin (`self.StartPosVLeft`)) false false))))
          (:`then_1`
            (bind (_direction_2 _rotate) (`Timeline|LeftValveRot`)
              (:`Update`
                (`SceneComponent.K2_SetRelativeRotation` (`self.ValveLeft`) (`KismetMathLibrary.MakeRotator` _startrotvleft_roll_2 (+ _rotate _startrotvleft_pitch_2) _startrotvleft_yaw_2) false false)
                ;[1 0.6864 0.09728] Sparks
                (`KismetSystemLibrary.Delay` 5.0)
                (set `self.randomFlickerValue` (`KismetMathLibrary.RandomInteger` 2))
                (if (== (`self.randomFlickerValue`) 0)
                  (`KismetSystemLibrary.Delay` (`KismetMathLibrary.RandomFloatInRange` 0.01 0.35))
                  (else
                    (`KismetSystemLibrary.Delay` (`KismetMathLibrary.RandomFloatInRange` 1.0 2.0))))
                (`ActorComponent.ToggleActive` (`self.SparksLeft`)))))))
      (:`then_1`
        (`|ExecutionSequence`
          (:`then_0`
            (bind (_direction_3 _plugin_2) (`Timeline|RightValveIn`)
              (:`Update`
                (`SceneComponent.K2_SetRelativeLocation` (`self.ValveRight`) (+ _plugin_2 (`self.StartPosVRight`)) false false))))
          (:`then_1`
            (bind (_direction_4 _rotate_2) (`Timeline|RightValveRot`)
              (:`Update`
                (`SceneComponent.K2_SetRelativeRotation` (`self.ValveRight`) (`KismetMathLibrary.MakeRotator` _startrotvleft_roll (+ _rotate_2 _startrotvleft_pitch) _startrotvleft_yaw) false false)
                (`KismetSystemLibrary.Delay` 5.0)
                (set `self.randomFlickerValue` (`KismetMathLibrary.RandomInteger` 2))
                (if (== (`self.randomFlickerValue`) 0)
                  (`KismetSystemLibrary.Delay` (`KismetMathLibrary.RandomFloatInRange` 0.01 0.35))
                  (else
                    (`KismetSystemLibrary.Delay` (`KismetMathLibrary.RandomFloatInRange` 1.0 2.0))))
                (`ActorComponent.ToggleActive` (`self.SparksRight`)))))))
      (:`then_2`
        ;[1 1 1] Panels
        (`|ExecutionSequence`
          (:`then_0`
            (bind (_direction_5 _doorstate) (`Timeline|Timeline_0`)
              (:`Update`
                (`SceneComponent.K2_SetRelativeLocation` (`self.PanelRight`) (+ _doorstate (`self.StartPosPRight`)) false false))))
          (:`then_1`
            (bind (_direction_6 _doorstate_2) (`Timeline|Timeline_1`)
              (:`Update`
                (`SceneComponent.K2_SetRelativeLocation` (`self.PanelLeft`) (+ _doorstate_2 (`self.StartPosPLeft`)) false false)))))))))

(fn `UserConstructionScript`)