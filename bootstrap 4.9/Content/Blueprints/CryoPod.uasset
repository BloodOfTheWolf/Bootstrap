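; CryoPod is a pod with two hinged doors that swing open when a ThirdPersonCharacter1 enters its trigger and close when it leaves.
; Two timelines add yaw to the hinge rotations cached at BeginPlay, staggered so the right door leads on opening and the left on closing.
; Closing requires the Open flag, which the left door's timeline update sets and nothing clears.
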(event `self.ReceiveBeginPlay`
  (set `self.left Hinge Start` (`SceneComponent.RelativeRotation` (`self.Left HInge`)))
  (set `self.Right Hinge Start` (`SceneComponent.RelativeRotation` (`self.Right Hinge`))))

(event `self.Trigger.OnComponentBeginOverlap`
  (params (OtherActor :type "Actor Object Reference") (OtherComp :type "PrimitiveComponent Object Reference") (OtherBodyIndex :type Integer) (bFromSweep :type Boolean) (SweepResult :type "HitResult Structure (by ref)"))
  (bind (_left_hinge_start_roll _left_hinge_start_pitch _left_hinge_start_yaw) (`KismetMathLibrary.BreakRotator` (`self.left Hinge Start`)))
  (bind (_right_hinge_start_roll _right_hinge_start_pitch _right_hinge_start_yaw) (`KismetMathLibrary.BreakRotator` (`self.Right Hinge Start`)))
  (if (`KismetMathLibrary.ClassIsChildOf` (`GameplayStatics.GetObjectClass` OtherActor) "/Game/ThirdPersonBP/Blueprints/ThirdPersonCharacter1.ThirdPersonCharacter1_C")
    (`|ExecutionSequence`
      (:`then_0`
        (`KismetSystemLibrary.Delay` 1.5)
        (bind (_direction _rotate) (`Timeline|Left Door` :!label _label)
          (:`Update`
            (`SceneComponent.K2_SetRelativeRotation` (`self.Left HInge`) (`KismetMathLibrary.MakeRotator` 0.0 0.0 (+ _rotate _left_hinge_start_yaw)) false false)
            (set `self.Open` true))))
      (:`then_1`
        (bind (_direction_2 _rotate_2) (`Timeline|RightDoor` :!label _label_2)
          (:`Update`
            (`SceneComponent.K2_SetRelativeRotation` (`self.Right Hinge`) (`KismetMathLibrary.MakeRotator` 0.0 0.0 (+ _rotate_2 _right_hinge_start_yaw)) false false)))))))

(event `self.Trigger.OnComponentEndOverlap`
  (params (OtherActor :type "Actor Object Reference") (OtherComp :type "PrimitiveComponent Object Reference") (OtherBodyIndex :type Integer))
  (if (`KismetMathLibrary.ClassIsChildOf` (`GameplayStatics.GetObjectClass` OtherActor) "/Game/ThirdPersonBP/Blueprints/ThirdPersonCharacter1.ThirdPersonCharacter1_C")
    (if (`self.Open`)
      (`|ExecutionSequence`
        (:`then_0`
          (goto _label :!via `Reverse`))
        (:`then_1`
          (`KismetSystemLibrary.Delay` 1.2)
          (goto _label_2 :!via `Reverse`))))))

(fn `UserConstructionScript`)